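; BP_Pickup is an inventory item pickup that displays the mesh of the item it represents.
; On BeginPlay and when its ID replicates, OnRep_ID looks up DT_Inventory and, if the row exists, sets Item to that row or to DropItem when that has an ID.
; Update then blocking-loads the item's pickup asset as a skeletal mesh, falling back to its static mesh.
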(event Custom|Update
  (bind _item (Variables|Default|GetItem))
  (bind (_pickup _staticpickup) (Utilities|Struct|BreakST_Inventory_Item _item))
  (bind _returnvalue (Utilities|LoadAssetBlocking _pickup))
  (bind _asskeletal_mesh (Utilities|Casting|CastToSkeletalMesh _returnvalue)
    (:then
      (Components|SkeletalMesh|SetSkeletalMeshAsset (Variables|Default|GetSkeletalMesh) _asskeletal_mesh))
    (:CastFailed
      (bind _returnvalue_2 (Utilities|LoadAssetBlocking _staticpickup))
      (bind _asstatic_mesh (Utilities|Casting|CastToStaticMesh _returnvalue_2))
      (Components|StaticMesh|SetStaticMesh (Variables|Default|GetStaticMesh) _asstatic_mesh))))

(event EventBeginPlay
  (CallFunction|OnRepID))

(fn ConstructionScript)

(fn OnRepID
  (bind _returnvalue (Utilities|GetDataTableRow "/Game/Elian/Inventory/DT_Inventory.DT_Inventory" (Variables|Default|GetID))
    (:then
      (Variables|Default|SetItem (select (!= (Utilities|Struct|BreakST_Inventory_Item (Variables|Default|GetDropItem)) "") (Variables|Default|GetDropItem) _returnvalue))
      (CallFunction|Update))))