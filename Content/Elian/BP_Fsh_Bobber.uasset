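; Fishing bobber actor that hooks and reels in trash, with a cable attached to the player that resizes to their distance each tick.
; Its first hit starts a random timer for a bite, and hooking spawns a BP_Trash and plays a bobbing timeline.
; Mouse wheel input feeds the reeling-game widget and pulls the bobber toward the player.
; Close range shows the collected-trash widget, while excess tension breaks the line, destroying catch and bobber.
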(event Custom|Hooked%20Fish
  (Variables|Default|SetFishHooked true)
  (bind _returnvalue (Game|SpawnActorfromClass "/Game/Elian/BP_Trash.BP_Trash_C" (Transformation|GetActorTransform) "Undefined" "MultiplyWithRoot" 0 0))
  (Variables|Default|SetFishCaught _returnvalue)
  (bind _bobfishon (Timeline|FISHON Play)
    (:Update
      (Transformation|SetRelativeLocation (Variables|Default|GetBobber) (* "0.000000,0.000000,20.000000" _bobfishon) false false))))

(event Custom|BreakLine
  ;[0.15 0.15 0.15 0.5] break the line if the tension is too strong
  (Actor|DestroyActor (Variables|Default|GetFishCaught))
  (Actor|DestroyActor))

(event Custom|TrashCaught
  (bind _returnvalue (UserInterface|CreateWidget "/Game/Elian/Widget/W_TrashCollected.W_TrashCollected_C" 0 (Variables|/Game/Elian/BP_Trash.BP_Trash_C|Getweight (Variables|Default|GetFishCaught))))
  (UserInterface|Viewport|AddtoViewport _returnvalue 0)
  (Utilities|FlowControl|Delay 0.6)
  (Actor|DestroyActor))

(event EventBeginPlay
  (Input|EnableInput (Game|GetPlayerController 0))
  (bind _asw_reeling_game (Utilities|Casting|CastToW_reelingGame (UserInterface|GetWidget (Variables|Default|GetReelGame))))
  (bind _output_get (Variables|Default|SetAs%20W%20Reeling%20Game _asw_reeling_game))
  (EventDispatchers|BindEventtoOnTensionMax _output_get (EventDispatchers|CreateEvent :!event Custom|BreakLine))
  (Class|CableComponent|SetAttachEndtoComponent (Variables|Default|GetCable) (Variables|/Script/Engine.Actor|GetRootComponent (Game|GetPlayerCharacter 0)) "None"))

(event Collision|EventActorBeginOverlap
  (params (OtherActor :type Actor%20Object%20Reference)))

(event Collision|EventHit
  (params (MyComp :type Primitive%20Component%20Object%20Reference) (Other :type Actor%20Object%20Reference) (OtherComp :type Primitive%20Component%20Object%20Reference) (bSelfMoved :type Boolean) (HitLocation :type Vector :default "0, 0, 0") (HitNormal :type Vector :default "0, 0, 0") (NormalImpulse :type Vector :default "0, 0, 0") (Hit :type Hit%20Result%20Structure%20%28by%20ref%29))
  (Utilities|FlowControl|DoOnce false
    (:Completed
      (Utilities|Time|SetTimerbyEvent (EventDispatchers|CreateEvent :!event Custom|Hooked%20Fish) (Math|Random|RandomFloatinRange 3.0 6.0)))))

(event EventTick
  (params (DeltaSeconds :type Float%20%28single-precision%29))
  (Variables|/Script/CableComponent.CableComponent|SetCableLength (Variables|Default|GetCable) (Math|Vector|Distance(Vector) (Transformation|GetActorLocation) (Transformation|GetActorLocation (Game|GetPlayerCharacter 0)))))

(event Input|MouseEvents|MouseWheelAxis
  (params (AxisValue :type Float%20%28single-precision%29))
  ;[0.15 0.15 0.15 0.5] check to see if mouse is inputing movement
  (if (Variables|Default|GetFishHooked)
    (bind _output_get (Variables|/Game/Elian/Widget/W_reelingGame.W_reelingGame_C|SetMouseMovement (Variables|Default|GetAs%20W%20Reeling%20Game) (Utilities|Operators|Divide (Math|Vector|VectorLength (Math|Conversions|ToVector(Float) AxisValue)) (Class|Actor|GetInputAxisKeyValue) -7.0)))
    (Components|MoveComponentTo (Variables|Default|GetCapsule) (Math|Vector|Lerp(Vector) (Transformation|GetActorLocation) (Transformation|GetActorLocation (Game|GetPlayerCharacter 0)) (/ _output_get 5.0)) (Transformation|GetActorRotation) false false (Utilities|Time|GetWorldDeltaSeconds) false)
    (if (< (Math|Vector|Distance(Vector) (Transformation|GetActorLocation) (Transformation|GetActorLocation (Game|GetPlayerCharacter 0))) 1.5e+02)
      (CallFunction|TrashCaught))))

(fn ConstructionScript)