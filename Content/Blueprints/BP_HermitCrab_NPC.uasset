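; Hermit crab NPC that wanders to random reachable points and offers interaction when the player character comes near.
; Entering its interaction sphere shows an interaction widget and a mission dialogue menu and enables input; leaving removes only the interaction widget and disables input.
; The Q key only prints a debug message.
; It also holds fishing functions, uncalled here, that line-trace ahead for water and spawn a bobber.
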(event OnComponentEndOverlap(InteractionSphere)
  (params (OverlappedComponent :type Primitive%20Component%20Object%20Reference) (OtherActor :type Actor%20Object%20Reference) (OtherComp :type Primitive%20Component%20Object%20Reference) (OtherBodyIndex :type Integer))
  ;[0.15 0.15 0.15 0.5] BP_Text_Interaction
  (bind _asbp_third_person_character (Utilities|Casting|CastToBP_ThirdPersonCharacter OtherActor))
  (Development|PrintString "no")
  (Variables|Default|SetCanInteract (== _asbp_third_person_character (Game|GetPlayerCharacter 0)))
  (Widget|RemovefromParent (Variables|Default|Getinteraction%20widget))
  ;;[0.15 0.15 0.15 0.5] allows this crabto listen for inputs
  (Input|DisableInput (Game|GetPlayerController 0)))

(event OnComponentBeginOverlap(InteractionSphere)
  (params (OverlappedComponent :type Primitive%20Component%20Object%20Reference) (OtherActor :type Actor%20Object%20Reference) (OtherComp :type Primitive%20Component%20Object%20Reference) (OtherBodyIndex :type Integer) (bFromSweep :type Boolean) (SweepResult :type Hit%20Result%20Structure%20%28by%20ref%29))
  ;[0.15 0.15 0.15 0.5] BP_Text_Interaction
  (bind _asbp_third_person_character (Utilities|Casting|CastToBP_ThirdPersonCharacter OtherActor))
  (Development|PrintString "Yes")
  (Variables|Default|SetCanInteract (== _asbp_third_person_character (Game|GetPlayerCharacter 0)))
  (UserInterface|Viewport|AddtoViewport (Variables|Default|Getinteraction%20widget) 0)
  ;;[0.15 0.15 0.15 0.5] allows this crabto listen for inputs
  (Input|EnableInput (Game|GetPlayerController 0))
  (bind _returnvalue (UserInterface|CreateWidget "/Game/Blueprints/BP_Dialogue_Menu_Mision.BP_Dialogue_Menu_Mision_C"))
  (UserInterface|Viewport|AddtoViewport _returnvalue 0))

(event Custom|Random%20Roam
  ;[0.15 0.15 0.15 0.5] NPC_Pedestrian_System
  (AI|AIMoveTo self (.RandomLocation (AI|Navigation|GetRandomReachablePointinRadius (Transformation|GetActorLocation) 2.5e+03 0 0)) 0 5.0 false
    (:OnSuccess
      (CallFunction|RandomRoam))))

(event EventBeginPlay
  ;[0.15 0.15 0.15 0.5] NPC_Pedestrian_System
  (CallFunction|RandomRoam)
  (bind _returnvalue (UserInterface|CreateWidget "/Game/Blueprints/BP_Interaction.BP_Interaction_C"))
  (Variables|Default|Setinteraction%20widget _returnvalue))

(event Input|KeyboardEvents|DebugKeyQ
  (params (Key :type Key%20Structure :default "None") (ActionValue :type Input%20Action%20Value%20Structure))
  ;[0.15 0.15 0.15 0.5] BP_Text_Interaction
  (:Pressed
    (Development|PrintString "interacting with crab")))

(fn ConstructionScript)

(fn CheckforWater
  (bind _returnvalue (Transformation|GetActorLocation))
  (bind _returnvalue_2 (Transformation|GetActorForwardVector))
  (bind _returnvalue_3 (Transformation|GetActorLocation))
  (bind _returnvalue_4 (Transformation|GetActorForwardVector))
  (bind _returnvalue_5 (* _returnvalue_2 4e+02))
  (bind _returnvalue_6 (* _returnvalue_4 4e+02))
  (bind _returnvalue_7 (+ _returnvalue _returnvalue_5))
  (bind _returnvalue_8 (+ _returnvalue_3 _returnvalue_6))
  ;[0.15 0.15 0.15 0.5] Checking Water
  (bind _returnvalue_9 (Collision|LineTraceByChannel _returnvalue_7 (+ _returnvalue_7 "0.000000,0.000000,-200.000000") "TraceTypeQuery1" false 0 "None"))
  (if (not _returnvalue_9)
    (bind _returnvalue_10 (Collision|LineTraceByChannel _returnvalue_8 (+ _returnvalue_8 "0.000000,0.000000,-200.000000") "TraceTypeQuery3" false 0 "ForOneFrame"))
    (bind _output_get (Variables|Default|SetCanFish _returnvalue_10))
    (return _output_get)))

(fn CastLine
  ;[0.15 0.15 0.15 0.5] Spawn Actor
  (bind _can_fish (CallFunction|CheckforWater))
  (if _can_fish
    (Game|SpawnActorfromClass "/Game/Elian/BP_Fsh_Bobber.BP_Fsh_Bobber_C" (Transformation|GetActorTransform) "AlwaysSpawn" "MultiplyWithRoot" self 0)))